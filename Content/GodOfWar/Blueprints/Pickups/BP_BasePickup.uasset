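; Base pickup actor for the God of War game that shows a world-space prompt and registers itself with Kratos for collection.
; An outer Proximity trigger toggles the widget, which turns toward the follow camera every tick.
; An inner Sphere trigger sets Kratos's CanPickup and Pickup reference and switches the widget's proximity state.
; TryCollectPickup and ReceivedAttribute are empty stubs, alongside a helper that spawns a pickup particle effect.
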(event `self.ReceiveBeginPlay`
  (bind _asbp_kratos (cast `/Game/GodOfWar/Blueprints/Character/BP_Kratos` (`GameplayStatics.GetPlayerCharacter` 0)))
  (set `self.BP Kratos` _asbp_kratos)
  (bind _asw_pickup (cast `/Game/GodOfWar/UI/W_Pickup` (`WidgetComponent.GetWidget` (`self.Widget`))))
  (set `self.W Pickup` _asw_pickup)
  (`SceneComponent.SetVisibility` (`self.Widget`) false false))

(event `self.ReceiveTick`
  (params (DeltaSeconds :type "Float (single-precision)"))
  (`/Engine/EditorBlueprintResources/StandardMacros.IsValid` (`self.BP Kratos`)
    (:`Is Valid`
      (`SceneComponent.K2_SetWorldRotation` (`self.Widget`) (`KismetMathLibrary.FindLookAtRotation` (`SceneComponent.K2_GetComponentLocation` (`self.Widget`)) (`SceneComponent.K2_GetComponentLocation` (`/Game/GodOfWar/Blueprints/Character/BP_Kratos.FollowCamera` (`self.BP Kratos`)))) false false))))

(event `Received Attribute`)

(event `self.Sphere.OnComponentBeginOverlap`
  (params (OverlappedComponent :type "PrimitiveComponent Object Reference") (OtherActor :type "Actor Object Reference") (OtherComp :type "PrimitiveComponent Object Reference") (OtherBodyIndex :type Integer) (bFromSweep :type Boolean) (SweepResult :type "HitResult Structure (by ref)"))
  (bind _w_pickup (`self.W Pickup`))
  (bind _asbp_kratos (cast `/Game/GodOfWar/Blueprints/Character/BP_Kratos` OtherActor))
  (set `/Game/GodOfWar/Blueprints/Character/BP_Kratos.CanPickup` true _asbp_kratos)
  (set `/Game/GodOfWar/Blueprints/Character/BP_Kratos.Pickup` self _asbp_kratos)
  (`/Engine/EditorBlueprintResources/StandardMacros.IsValid` _w_pickup
    (:`Is Valid`
      (`/Game/GodOfWar/UI/W_Pickup.SetProximity` _w_pickup false))))

(event `self.Sphere.OnComponentEndOverlap`
  (params (OverlappedComponent :type "PrimitiveComponent Object Reference") (OtherActor :type "Actor Object Reference") (OtherComp :type "PrimitiveComponent Object Reference") (OtherBodyIndex :type Integer))
  (bind _w_pickup (`self.W Pickup`))
  (bind _asbp_kratos (cast `/Game/GodOfWar/Blueprints/Character/BP_Kratos` OtherActor))
  (set `/Game/GodOfWar/Blueprints/Character/BP_Kratos.CanPickup` false _asbp_kratos)
  (set `/Game/GodOfWar/Blueprints/Character/BP_Kratos.Pickup` null _asbp_kratos)
  (`/Engine/EditorBlueprintResources/StandardMacros.IsValid` _w_pickup
    (:`Is Valid`
      (`/Game/GodOfWar/UI/W_Pickup.SetProximity` _w_pickup true))))

(event `self.Proximity.OnComponentBeginOverlap`
  (params (OverlappedComponent :type "PrimitiveComponent Object Reference") (OtherActor :type "Actor Object Reference") (OtherComp :type "PrimitiveComponent Object Reference") (OtherBodyIndex :type Integer) (bFromSweep :type Boolean) (SweepResult :type "HitResult Structure (by ref)"))
  (cast `/Game/GodOfWar/Blueprints/Character/BP_Kratos` OtherActor)
  (`SceneComponent.SetVisibility` (`self.Widget`) true false))

(event `self.Proximity.OnComponentEndOverlap`
  (params (OverlappedComponent :type "PrimitiveComponent Object Reference") (OtherActor :type "Actor Object Reference") (OtherComp :type "PrimitiveComponent Object Reference") (OtherBodyIndex :type Integer))
  (cast `/Game/GodOfWar/Blueprints/Character/BP_Kratos` OtherActor)
  (`SceneComponent.SetVisibility` (`self.Widget`) false false))

(fn `SpawnParticleOnPickedUp`
  (`GameplayStatics.SpawnEmitterAtLocation` (`self.Emitter Template`) (`SceneComponent.K2_GetComponentLocation` (`self.DefaultSceneRoot`)) (struct) (0.7 0.7 0.7)))

(fn `TryCollectPickup`)

(fn `UserConstructionScript`)