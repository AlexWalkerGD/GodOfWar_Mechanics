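; Thrown axe projectile that sticks where it hits and can be recalled to the player, God of War style.
; Each tick, a one-unit world-X trace from the axe head stops its movement, spin and gravity on the first blocking hit.
; A one-shot Return event eases the axe to the character mesh's transform, destroys it and calls VisibleAxe on the character.
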(event `self.ReceiveTick`
  (params (DeltaSeconds :type "Float (single-precision)"))
  (bind _axe_head (`self.Axe Head`))
  (bind _projectilemovement (`self.ProjectileMovement`))
  (bind (_returnvalue_x _returnvalue_y _returnvalue_z) (`KismetMathLibrary.BreakVector` (`SceneComponent.K2_GetComponentLocation` _axe_head)))
  (bind _outhit (`KismetSystemLibrary.LineTraceSingle` (`SceneComponent.K2_GetComponentLocation` _axe_head) (`KismetMathLibrary.MakeVector` (+ _returnvalue_x 1.0) _returnvalue_y _returnvalue_z) "TraceTypeQuery1"))
  (if (`GameplayStatics.BreakHitResult` _outhit)
    (`/Engine/EditorBlueprintResources/StandardMacros.DoOnce` false
      (:`Completed`
        (`MovementComponent.StopMovementImmediately` _projectilemovement)
        (set `RotatingMovementComponent.RotationRate` (struct) (`self.RotatingMovement`))
        (set `ProjectileMovementComponent.ProjectileGravityScale` 0.0 _projectilemovement)))))

(event `Return`
  (`/Engine/EditorBlueprintResources/StandardMacros.DoOnce` false
    (:`Completed`
      (bind _asbp_third_person_character (cast `/Game/ThirdPerson/Blueprints/BP_ThirdPersonCharacter` (`GameplayStatics.GetPlayerCharacter` 0)))
      (bind (_returnvalue_location _returnvalue_rotation) (`KismetMathLibrary.BreakTransform` (`SceneComponent.K2_GetComponentToWorld` (`Character.Mesh` _asbp_third_person_character))))
      (`KismetSystemLibrary.MoveComponentTo` (`self.DefaultSceneRoot`) _returnvalue_location _returnvalue_rotation false true 0.3)
      (`self.K2_DestroyActor`)
      (`/Game/ThirdPerson/Blueprints/BP_ThirdPersonCharacter.Visible Axe` _asbp_third_person_character))))

(fn `UserConstructionScript`)