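; Actor component that tracks an actor's health, death state and a Fury resource, with getters for raw and normalized values.
; Clamped functions apply damage, healing and Fury changes, setting death at zero health and ending Fury mode when nearly empty.
; RepNotify variables fire health, Fury and death dispatchers.
; Recovery checks compare against a hardcoded 100 rather than the Max variables, and healing ignores the death state.
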(fn `ApplyDamage`
  (params (Damage :type "Float (double-precision)"))
  (if (`self.CanReceiveDamage`)
    (bind _output_get (set `self.Health` (`KismetMathLibrary.FClamp` (- (`self.Health`) (`local.Damage`)) 0.0 (`self.Max Health`))))
    (if (<= _output_get 0.0)
      (set `self.IsDead` true))))

(fn `ApplyFury`
  (params (ConsumeFury :type "Float (double-precision)"))
  (if (`self.OnFury`)
    (if (`self.CanUseFury`)
      (bind _output_get (set `self.Fury` (`KismetMathLibrary.FClamp` (- (`self.Fury`) (`local.ConsumeFury`)) 0.0 (`self.MaxFury`))))
      (if (<= _output_get 1.0)
        (set `self.OnFury` false)))))

(fn `CanReceiveDamage`
  (returns (Return :type Boolean))
  (return (not (`self.IsDead`))))

(fn `CanReceiveFury`
  (returns (Return :type Boolean))
  (return (< (`self.Fury`) 100.0)))

(fn `CanReceiveHealth`
  (returns (ReturnValue :type Boolean))
  (return (< (`self.Health`) 100.0)))

(fn `CanUseFury`
  (returns (Return :type Boolean))
  (return (> (`self.Fury`) 1.0)))

(fn `GetDeadState`
  (returns (IsDead :type Boolean))
  (return (`self.IsDead`)))

(fn `GetFury`
  (returns (Fury :type "Float (double-precision)"))
  (return (`self.Fury`)))

(fn `GetHealth`
  (returns (Health :type "Float (double-precision)"))
  (return (`self.Health`)))

(fn `GetNormalizadFury`
  (returns (NormalizedFury :type "Float (double-precision)"))
  (return (/ (`self.Fury`) (`self.MaxFury`))))

(fn `GetNormalizadHealth`
  (returns (NormalizedHealth :type "Float (double-precision)"))
  (return (/ (`self.Health`) (`self.Max Health`))))

(fn `OnRep_Fury`
  (`self.OnFuryChange` self))

(fn `OnRep_Health`
  (`self.OnHealthChange` self))

(fn `OnRep_IsDead`
  (`self.OnDied`))

(fn `OnRep_Max Health`)

(fn `RecoverFury`
  (params (`Add Fury` :type "Float (double-precision)"))
  (if (`self.CanReceiveFury`)
    (set `self.Fury` (`KismetMathLibrary.FClamp` (+ (`self.Fury`) (`local.Add Fury`)) 0.0 (`self.MaxFury`)))))

(fn `RecoverHealth`
  (params (`Add Health` :type "Float (double-precision)"))
  (if (`self.CanReceiveHealth`)
    (set `self.Health` (`KismetMathLibrary.FClamp` (+ (`self.Health`) (`local.Add Health`)) 0.0 (`self.Max Health`)))))