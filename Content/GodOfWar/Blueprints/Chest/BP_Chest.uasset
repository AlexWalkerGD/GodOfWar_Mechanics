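; BP_Chest is an interactable chest that Kratos can open, with a spell bag spawned at its spawn point on BeginPlay.
; A Proximity volume shows a camera-facing pickup widget, while the inner Box updates that widget and registers the chest on Kratos as openable.
; BrokenSkull sets physics on the skull Geometry Collection, then removes the thunder-ball component and widget, disables further overlap handling and plays the open animation.
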(event `self.ReceiveBeginPlay`
  (bind _asbp_kratos (cast `/Game/GodOfWar/Blueprints/Character/BP_Kratos` (`GameplayStatics.GetPlayerCharacter` 0)))
  (set `self.BP Kratos` _asbp_kratos)
  (bind _asw_pickup (cast `/Game/GodOfWar/UI/W_Pickup` (`WidgetComponent.GetWidget` (`self.Widget`))))
  (set `self.W Pickup` _asw_pickup)
  (`SceneComponent.SetVisibility` (`self.Widget`) false false)
  (`self.SpawnSpellBag`))

(event `self.ReceiveTick`
  (params (DeltaSeconds :type "Float (single-precision)"))
  (bind _widget (`self.Widget`))
  (`/Engine/EditorBlueprintResources/StandardMacros.IsValid` (`self.BP Kratos`)
    (:`Is Valid`
      (`/Engine/EditorBlueprintResources/StandardMacros.IsValid` _widget
        (:`Is Valid`
          (`SceneComponent.K2_SetWorldRotation` (`self.Widget`) (`KismetMathLibrary.FindLookAtRotation` (`SceneComponent.K2_GetComponentLocation` _widget) (`SceneComponent.K2_GetComponentLocation` (`/Game/GodOfWar/Blueprints/Character/BP_Kratos.FollowCamera` (`self.BP Kratos`)))) false false))))))

(event `self.Box.OnComponentBeginOverlap`
  (params (OverlappedComponent :type "PrimitiveComponent Object Reference") (OtherActor :type "Actor Object Reference") (OtherComp :type "PrimitiveComponent Object Reference") (OtherBodyIndex :type Integer) (bFromSweep :type Boolean) (SweepResult :type "HitResult Structure (by ref)"))
  (bind _w_pickup (`self.W Pickup`))
  (if (`self.IsNotInvalid`)
    (bind _asbp_kratos (cast `/Game/GodOfWar/Blueprints/Character/BP_Kratos` OtherActor))
    (set `/Game/GodOfWar/Blueprints/Character/BP_Kratos.CanOpenChest` true _asbp_kratos)
    (set `/Game/GodOfWar/Blueprints/Character/BP_Kratos.Chest` self _asbp_kratos)
    (`/Engine/EditorBlueprintResources/StandardMacros.IsValid` _w_pickup
      (:`Is Valid`
        (`/Game/GodOfWar/UI/W_Pickup.SetProximity` _w_pickup false)))))

(event `self.Box.OnComponentEndOverlap`
  (params (OverlappedComponent :type "PrimitiveComponent Object Reference") (OtherActor :type "Actor Object Reference") (OtherComp :type "PrimitiveComponent Object Reference") (OtherBodyIndex :type Integer))
  (bind _w_pickup (`self.W Pickup`))
  (if (`self.IsNotInvalid`)
    (bind _asbp_kratos (cast `/Game/GodOfWar/Blueprints/Character/BP_Kratos` OtherActor))
    (set `/Game/GodOfWar/Blueprints/Character/BP_Kratos.CanOpenChest` false _asbp_kratos)
    (set `/Game/GodOfWar/Blueprints/Character/BP_Kratos.Chest` null _asbp_kratos)
    (`/Engine/EditorBlueprintResources/StandardMacros.IsValid` _w_pickup
      (:`Is Valid`
        (`/Game/GodOfWar/UI/W_Pickup.SetProximity` _w_pickup true)))))

(event `self.Proximity.OnComponentBeginOverlap`
  (params (OverlappedComponent :type "PrimitiveComponent Object Reference") (OtherActor :type "Actor Object Reference") (OtherComp :type "PrimitiveComponent Object Reference") (OtherBodyIndex :type Integer) (bFromSweep :type Boolean) (SweepResult :type "HitResult Structure (by ref)"))
  (if (`self.IsNotInvalid`)
    (cast `/Game/GodOfWar/Blueprints/Character/BP_Kratos` OtherActor)
    (`SceneComponent.SetVisibility` (`self.Widget`) true false)))

(event `self.Proximity.OnComponentEndOverlap`
  (params (OverlappedComponent :type "PrimitiveComponent Object Reference") (OtherActor :type "Actor Object Reference") (OtherComp :type "PrimitiveComponent Object Reference") (OtherBodyIndex :type Integer))
  (if (`self.IsNotInvalid`)
    (cast `/Game/GodOfWar/Blueprints/Character/BP_Kratos` OtherActor)
    (`SceneComponent.SetVisibility` (`self.Widget`) false false)))

(fn `BrokenSkull`
  (params (bSimulate :type Boolean))
  (bind _p_ky_thunderball (`self.P_ky_thunderBall`))
  (`PrimitiveComponent.SetSimulatePhysics` (`self.skull_GeometryCollection`) bSimulate)
  (`/Engine/EditorBlueprintResources/StandardMacros.IsValid` _p_ky_thunderball
    (:`Is Valid`
      (`/Engine/EditorBlueprintResources/StandardMacros.IsValid` (`self.Widget`)
        (:`Is Valid`
          (`ActorComponent.K2_DestroyComponent` _p_ky_thunderball)
          (`ActorComponent.K2_DestroyComponent` (`self.Widget`))
          (set `self.IsNotInvalid` false)
          (`SkeletalMeshComponent.PlayAnimation` (`self.Chest`) "/Game/GodOfWar/Blueprints/Chest/source/Chest_Anim_Armature_A_Open.Chest_Anim_Armature_A_Open" false))))))

(fn `SpawnSpellBag`
  (bind (_returnvalue_location _returnvalue_rotation) (`KismetMathLibrary.BreakTransform` (`SceneComponent.K2_GetComponentToWorld` (`self.PointToSpawn`))))
  (bind _returnvalue (`|SpawnActorFromClass` "/Game/GodOfWar/Blueprints/Chest/BP_SpellBag.BP_SpellBag_C" (`KismetMathLibrary.MakeTransform` _returnvalue_location _returnvalue_rotation) "Undefined" "MultiplyWithRoot" null null))
  (set `self.SpellBag` _returnvalue))

(fn `UserConstructionScript`)